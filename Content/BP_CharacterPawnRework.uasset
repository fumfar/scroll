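; Character pawn for an idle RPG that passively earns experience and gold, levels up and shows the UserInterface widget.
; BeginPlay requests an IdleSave load and copies CharacterStructure into its stat variables.
; Tick detects real-time second changes to regenerate MP, test level-up (raising stats and a quadratic EXP threshold) and add income.
; It then packs stats into a newly created IdleSave each second, without writing it to a slot.
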(event EventBeginPlay
  (bind _returnvalue (UserInterface|CreateWidget "/Game/Widgets/UserInterface.UserInterface_C"))
  (bind _output_get (Variables|Misc|SetUIReference _returnvalue))
  (UserInterface|Viewport|AddtoViewport _output_get 0)
  (Utilities|UpdateCharacterBlueprint))

(event Collision|EventActorBeginOverlap
  (params (OtherActor :type Actor%20Object%20Reference)))

(event EventTick
  (params (DeltaSeconds :type Float%20%28single-precision%29))
  (Utilities|HasASecondPassed
    (:Out
      (Utilities|RegenerateMP)
      (Utilities|LevelUpTest
        (:HasLeveled
          (Utilities|CurrentLevel+)
          (Utilities|ExptoNextLevelFunction
            (:Out
              _)))
        (:NotLeveled
          _))
      (CallFunction|GenerateExp)
      (CallFunction|GenerateCash)
      (Utilities|SaveCharacterStruct))))

(fn ConstructionScript)

(fn GenerateExp
  (if (== (Variables|Exp|GetCurrentLevel) 1)
    (Variables|Exp|SetExpToNext 100))
  (Utilities|AddExp
    (:o
      (return))))

(fn GenerateCash
  (Variables|Gold|SetCurrentGold (+ (Variables|Gold|GetCurrentGold) (Variables|Gold|GetGoldPerSecond)))
  (return))

(fn GenerateItem)