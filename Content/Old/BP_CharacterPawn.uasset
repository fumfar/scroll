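; Character pawn for an idle-RPG-style progression loop that creates the UserInterface widget and earns gold and experience over time.
; Tick uses a once-per-second gate to run the level-up check, roll random gold, compute stat-based experience and rebuild CharacterStructure, printing debug values.
; The progression is unfinished: the experience formulas are unwired, exp-to-next outputs return zero, LevelUp is empty and the random equipment drop roll is never called.
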(event EventBeginPlay
  (bind _returnvalue (UserInterface|CreateWidget "/Game/Widgets/UserInterface.UserInterface_C"))
  (bind _output_get (Variables|UMG|SetInterface _returnvalue))
  (UserInterface|Viewport|AddtoViewport _output_get 0))

(event Collision|EventActorBeginOverlap
  (params (OtherActor :type Actor%20Object%20Reference)))

(event EventTick
  (params (DeltaSeconds :type Float%20%28single-precision%29))
  (bind _characterstructure (Variables|Save|GetCharacterStructure))
  (bind (_level _tech _skill _def _luck _faith _exp) (Utilities|Struct|BreakCharacterStructure _characterstructure))
  (bind _output_get (Utilities|GetGameTimeinSeconds))
  (Utilities|HasSecondPassed _output_get
    (:Second%20Has%20Passed
      (Utilities|HasLeveledUp
        (:out
          (bind (_currentgold _alltimegold) (CallFunction|GenerateCash))
          (bind (_exp_2 _level_2 _exptonext) (CallFunction|GenerateExp (Variables|Exp|GetCurrentLevel)))
          (CallFunction|UpdateCharacter _level_2 _exp_2 _currentgold _alltimegold _exptonext)
          (for _array_element (Utilities|Array|MakeArray _level _exp _exptonext)
            (Development|PrintString (Utilities|String|ToString(Integer) _array_element) true true "(R=0.000000,G=0.660000,B=1.000000,A=1.000000)" 1.0)))))))

(fn ConstructionScript)

(fn GenerateCash
  (bind _characterstructure (Variables|Save|GetCharacterStructure))
  (bind (_level _tech _skill _def _luck _faith _exp _expper _cash _cashper _cost _gametime _alltimecash) (Utilities|Struct|BreakCharacterStructure _characterstructure))
  (bind _output_get (LocalVariables|SetNewLocalVar_0 (Math|Float|Round (Math|Random|RandomFloatinRange (* _cashper (* _cost 0.05)) (Math|Conversions|ToFloat(Integer) _cashper)))))
  (bind _output_get_2 (Variables|Gold|SetCurrentGold (+ (Variables|Gold|GetCurrentGold) _output_get)))
  (bind _output_get_3 (Variables|Gold|SetAllTimeGold (+ _output_get _alltimecash)))
  (return _output_get_2 _output_get_3))

(fn GenerateExp
  (params (CurrentLevel :type Integer))
  (bind _characterstructure (Variables|Save|GetCharacterStructure))
  (bind (_level _tech _skill _def _luck _faith _exp _expper) (Utilities|Struct|BreakCharacterStructure _characterstructure))
  (bind _output_get (Variables|Exp|SetCurrentLevel CurrentLevel))
  (bind _output_get_2 (Variables|Exp|SetCurrentExp (Utilities|ExpEquation _expper _skill _def _luck _faith 0 _tech _exp 0)))
  (return _output_get_2 _output_get 0))

(fn UpdateCharacter
  (params (LEVEL :type Integer) (EXP :type Integer) (CASH :type Integer) (ALLTIMECASH :type Integer) (exp%20to%20next%20level :type Integer) (SCROLLDROP :type Scroll%20Structure%20Structure) (EQUIPMENTDROP :type Item%20Structure%20Structure))
  (Variables|Save|SetCharacterStructure (Utilities|Struct|MakeCharacterStructure LEVEL 20 2 2 2 2 EXP 10 CASH 20 2 0 ALLTIMECASH (Variables|Inventory|GetEquipmentInventory) (Variables|Inventory|GetScrollInventory) "(HP_18_2425D41A4D62D34BD013A5BAC81CD49A=0,MP_19_9CDADDDB46AD9B38CDF20FA6BF3E35A0=0,SKILL_20_6B1DBF5D45DE1832A214CEA43C718ED8=0,DEF_21_B759FBE047AF5DCE02EAF9AFEAC97F73=0,LUCK_22_488F52DD467854EC87E1EF9FBE9DD5D8=0,FAITH_23_FC8549114DA9323F6A360EB9F145310D=0,ITEMLEVEL_24_955A0E4E49AF4420BF049BBD7A6E077E=0,SLOTS_25_12135B514A193D3E1A4293968755EDB0=0,ITEMTYPE_26_96345A2C4A9281A1CF9EAC9C6399281B=NewEnumerator0,BASEVALUE_31_7368BD3B492C694E56B6F69535A08864=0,CURRENTVALUE_32_40897ACD4EE7A8A9FA921A9D61645538=0)")))

(fn RollforDrop
  (if (== (Math|Random|RandomIntegerinRange 0 1) 1)
    (if (== (Math|Random|RandomIntegerinRange 0 1) 0)
      (Utilities|Array|Add (Variables|Inventory|GetEquipmentInventory) (Variables|Items|GetItemStructure))))
  (return "" ""))